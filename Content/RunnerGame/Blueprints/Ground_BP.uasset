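; Ground_BP is an endless-runner ground segment that, on BeginPlay, fills five rows of three arrow markers with obstacles.
; Each row randomly gets one or two Obsticle_BP actors, with a chance to replace them with another spawn whose class is unset here.
; When the player overlaps Box, it spawns the next segment at ArrowEnd and destroys itself after a delay.
; Box1 calls the character's Death as a fall-out-of-map trigger.
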(event `self.ReceiveBeginPlay`
  ;[1 1 1] Refrense and Obstacle Spawn
  (`self.Obstacle Spawn` (`self.Arrow_Obstacle_01`) (`self.Arrow_Obstacle_02`) (`self.Arrow_Obstacle_03`))
  (`self.Obstacle Spawn` (`self.Arrow_Obstacle_04`) (`self.Arrow_Obstacle_05`) (`self.Arrow_Obstacle_06`))
  (`self.Obstacle Spawn` (`self.Arrow_Obstacle_07`) (`self.Arrow_Obstacle_08`) (`self.Arrow_Obstacle_09`))
  (`self.Obstacle Spawn` (`self.Arrow_Obstacle_010`) (`self.Arrow_Obstacle_011`) (`self.Arrow_Obstacle_012`))
  (`self.Obstacle Spawn` (`self.Arrow_Obstacle_013`) (`self.Arrow_Obstacle_014`) (`self.Arrow_Obstacle_015`)))

(event `self.Box.OnComponentBeginOverlap`
  (params (OverlappedComponent :type "PrimitiveComponent Object Reference") (OtherActor :type "Actor Object Reference") (OtherComp :type "PrimitiveComponent Object Reference") (OtherBodyIndex :type Integer) (bFromSweep :type Boolean) (SweepResult :type "HitResult Structure (by ref)"))
  ;[1 1 1] Ground Spawn and Destroy
  (cast `/Game/RunnerGame/Blueprints/BP_ThirdPersonCharacter` OtherActor)
  (`|SpawnActorFromClass` "Ground_BP_C" (`SceneComponent.K2_GetComponentToWorld` (`self.ArrowEnd`)) "Undefined" "OverrideRootScale" null null)
  (`KismetSystemLibrary.Delay` 25.0)
  (`self.K2_DestroyActor`))

(event `self.Box1.OnComponentBeginOverlap`
  (params (OverlappedComponent :type "PrimitiveComponent Object Reference") (OtherActor :type "Actor Object Reference") (OtherComp :type "PrimitiveComponent Object Reference") (OtherBodyIndex :type Integer) (bFromSweep :type Boolean) (SweepResult :type "HitResult Structure (by ref)"))
  ;[1 1 1] When fall out map Die
  (bind _asbp_third_person_character (cast `/Game/RunnerGame/Blueprints/BP_ThirdPersonCharacter` OtherActor))
  (`/Game/RunnerGame/Blueprints/BP_ThirdPersonCharacter.Death` _asbp_third_person_character))

(fn `New Function`)

(fn `Obstacle Spawn`
  (params (`[0]` :type "ArrowComponent Object Reference") (`[1]` :type "ArrowComponent Object Reference") (`[2]` :type "ArrowComponent Object Reference"))
  (bind _returnvalue (`KismetMathLibrary.Conv_VectorToTransform` (`SceneComponent.K2_GetComponentLocation` (`|GetArrayItem` (`|MakeArray` `[0]` `[1]` `[2]`) (`KismetMathLibrary.RandomIntegerInRange` 0 2)))))
  (bind _returnvalue_2 (`|SpawnActorFromClass` "/Game/RunnerGame/Blueprints/Obsticle_BP.Obsticle_BP_C" _returnvalue "Undefined" "OverrideRootScale" null null))
  (if (`KismetMathLibrary.RandomBool`)
    (bind _returnvalue_3 (`|SpawnActorFromClass` "/Game/RunnerGame/Blueprints/Obsticle_BP.Obsticle_BP_C" _returnvalue "Undefined" "OverrideRootScale" null null))
    (bind _output_get (set `self.X` 1))
    (bind _output_get_2 (set `self.Y` (`KismetMathLibrary.FTrunc` (`KismetMathLibrary.RandomFloatInRange` 1.0 9.0))))
    (bind _output_get_3 (set `self.TrueFalse` (== _output_get _output_get_2)))
    (if _output_get_3
      (`self.K2_DestroyActor` _returnvalue_3)
      (`self.K2_DestroyActor` _returnvalue_2)
      (`|SpawnActorFromClass` "/Game/RunnerGame/Blueprints/GiantPower_BP.GiantPower_BP_C" _returnvalue "Undefined" "OverrideRootScale" null null))
    (else
      (bind _output_get_4 (set `self.X` 1))
      (bind _output_get_5 (set `self.Y` (`KismetMathLibrary.FTrunc` (`KismetMathLibrary.RandomFloatInRange` 1.0 3.0))))
      (bind _output_get_6 (set `self.TrueFalse` (== _output_get_4 _output_get_5)))
      (if _output_get_6
        (`self.K2_DestroyActor` _returnvalue_2)
        (`|SpawnActorFromClass` "/Game/RunnerGame/Blueprints/Terrain_BP.Terrain_BP_C" _returnvalue "Undefined" "OverrideRootScale" null null)))))

(fn `UserConstructionScript`)