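; Camera actor for the runner game that tracks a followed actor along the X axis only.
; SetupFollowActor stores the target and captures the offset between the camera and that actor at that moment.
; Every Tick moves the camera to the target's X plus that offset, ignoring the target's Y and Z movement, with no sweep or smoothing.
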(event `self.ReceiveTick`
  (params (DeltaSeconds :type "Float (single-precision)"))
  (bind _returnvalue_x (`KismetMathLibrary.BreakVector` (`self.K2_GetActorLocation` (`self.Follow Actor`))))
  ;[1 1 1] Camera get Player Pos
  (`self.K2_SetActorLocation` (+ (`KismetMathLibrary.MakeVector` _returnvalue_x) (`self.Offset`))))

(fn `Setup Follow Actor`
  (params (Actor :type "Actor Object Reference"))
  (set `self.Follow Actor` Actor)
  (set `self.Offset` (- (`self.K2_GetActorLocation`) (`self.K2_GetActorLocation` Actor))))

(fn `UserConstructionScript`)